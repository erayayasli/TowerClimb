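; BP_Win is a finish-trigger actor that also runs the level's start countdown and timed-run flow.
; On BeginPlay it disables player input and ticks a countdown widget each second with a sound, then restores input and shows the timer widget.
; When BP_King overlaps its Box, it hides the timer, shows the recorded time on a win widget, and reloads the current level after a delay.
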(event `self.ReceiveBeginPlay`
  (bind _returnvalue (`|CreateWidget` "/Game/Widget/WBP_Timer.WBP_Timer_C"))
  (set `self.Timer` _returnvalue)
  (bind _returnvalue_2 (`|CreateWidget` "/Game/Widget/WBP_Countdown.WBP_Countdown_C"))
  (bind _output_get (set `self.CountdownWidget` _returnvalue_2))
  (`UserWidget.AddToViewport` _output_get 0)
  (bind _returnvalue_3 (`KismetSystemLibrary.K2_SetTimerDelegate` (delegate `TakeCountdown`) 1.0 true))
  (`self.DisableInput` (`GameplayStatics.GetPlayerCharacter` 0) (`GameplayStatics.GetPlayerController` 0)))

(event `TakeCountdown`
  (`/Engine/EditorBlueprintResources/StandardMacros.DecrementInt` (`self.Count`)
    (:`  `
      (`TextBlock.SetText` (`/Game/Widget/WBP_Countdown.CountdownText` (`self.CountdownWidget`)) (`KismetTextLibrary.Conv_IntToText` (`self.Count`)))
      (`GameplayStatics.PlaySound2D` "/Engine/VREditor/Sounds/UI/Camera_Shutter.Camera_Shutter" 1.0 1.0 0.0 null null)
      (if (<= (`self.Count`) 0)
        (`KismetSystemLibrary.K2_ClearAndInvalidateTimerHandle` (stale `self.ReceiveBeginPlay` _returnvalue_3))
        (`Widget.RemoveFromParent` (`self.CountdownWidget`))
        (`self.EnableInput` (`GameplayStatics.GetPlayerCharacter` 0) (`GameplayStatics.GetPlayerController` 0))
        (`UserWidget.AddToViewport` (`self.Timer`) 0)))))

(event `self.Box.OnComponentBeginOverlap`
  (params (OverlappedComponent :type "PrimitiveComponent Object Reference") (OtherActor :type "Actor Object Reference") (OtherComp :type "PrimitiveComponent Object Reference") (OtherBodyIndex :type Integer) (bFromSweep :type Boolean) (SweepResult :type "HitResult Structure (by ref)"))
  (bind _timer (`self.Timer`))
  (cast `/Game/Blueprints/Characters/King/BP_King` OtherActor)
  (bind _returnvalue (`GameplayStatics.GetCurrentLevelName` true))
  (`Widget.SetVisibility` _timer "Hidden")
  (bind _returnvalue_2 (`|CreateWidget` "/Game/Widget/WBP_Win.WBP_Win_C"))
  (`TextBlock.SetText` (`/Game/Widget/WBP_Win.TimeText` _returnvalue_2) (`KismetTextLibrary.Conv_DoubleToText` (`/Game/Widget/WBP_Timer.Time` _timer) "HalfToEven"))
  (`UserWidget.AddToViewport` _returnvalue_2 0)
  (`KismetSystemLibrary.Delay` 5.0)
  (`GameplayStatics.OpenLevel` (`KismetStringLibrary.Conv_StringToName` _returnvalue)))

(fn `ShowCountdown`
  (params (CoundownWidget :type "UserWidget Object Reference")))

(fn `UserConstructionScript`)